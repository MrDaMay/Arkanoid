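; Block spawner for level 1 that builds the grid of blocks and moves the game on to Level_2 once none are left.
; BeginPlay loops over X and Y, spawning scaled BP_CubeBLock1 actors at padded negative world offsets and incrementing LivesBlocks for each.
; Tick polls that counter and opens Level_2 at zero; nothing in this Blueprint decrements it.
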(event EventBeginPlay
  (Variables|Default|SetCheckLevel true)
  (for _index (range 1 (Variables|Default|GetX))
    (for _index_2 (range 1 (Variables|Default|GetY))
      (bind _result (Math|Integer|IncrementInt (Variables|Default|GetLivesBlocks))
        (:%20%20
          (Variables|Default|SetLivesBlocks _result)
          (Game|SpawnActorfromClass "/Game/Blueprints/BP_CubeBLock1.BP_CubeBLock1_C" (Math|Transform|MakeTransform (Math|Vector|MakeVector (Math|Conversions|ToFloat(Integer) (* (* _index (Variables|Default|GetPadding_X)) -1)) (Math|Conversions|ToFloat(Integer) (* (* _index_2 (Variables|Default|GetPadding_Y)) -1)) 0.0) "0, 0, 0" "1.400000,0.700000,0.700000") "Undefined" 0 0))))))

(event Collision|EventActorBeginOverlap
  (params (OtherActor :type Actor%20Object%20Reference)))

(event EventTick
  (params (DeltaSeconds :type Float%20%28single-precision%29))
  (if (== (Variables|Default|GetLivesBLocks) 0)
    (Game|OpenLevel(byName) "Level_2")))

(fn ConstructionScript)