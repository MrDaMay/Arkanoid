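; BP_Bonus1 is a moving bonus pickup that adds five points to the score when the player pawn touches it.
; On BeginPlay it caches the BP_Score game instance, then destroys itself when it overlaps either BP_Pawn or a KillZVolume.
; Each tick it spins its Cylinder1 component by a fixed per-frame step and moves along DirectionMove at Speed with a swept, delta-time-scaled local offset.
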(event EventBeginPlay
  (bind _asbp_score (Utilities|Casting|CastToBP_Score (Game|GetGameInstance)))
  (Variables|Default|SetScore _asbp_score))

(event Collision|EventActorBeginOverlap
  (params (OtherActor :type Actor%20Object%20Reference))
  (Utilities|Casting|CastToBP_Pawn OtherActor
    (:then
      (Variables|/Game/Blueprints/BP_Score.BP_Score_C|SetScore (Variables|Default|GetScore) (+ (Variables|/Game/Blueprints/BP_Score.BP_Score_C|GetScore (Variables|Default|GetScore)) 5))
      (Actor|DestroyActor))
    (:CastFailed
      (Utilities|Casting|CastToKillZVolume OtherActor)
      (Actor|DestroyActor))))

(event EventTick
  (params (DeltaSeconds :type Float%20%28single-precision%29))
  (Transformation|AddWorldRotation (Variables|Default|GetCylinder1) "0, 0,-10.000000" false false)
  (Transformation|AddActorLocalOffset (* (* (Variables|Default|GetDirectionMove) (Variables|Default|GetSpeed)) DeltaSeconds) true false))

(fn ConstructionScript)