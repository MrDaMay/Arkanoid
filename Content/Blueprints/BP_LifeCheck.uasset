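; BP_LifeCheck is a lives indicator that shows the player pawn's remaining lives as three groups of three cube components.
; BeginPlay stores the first BP_Pawn found, and Tick polls its Life value through nested threshold branches.
; At two, one and zero lives or below, the matching group is destroyed once, guarded by a boolean.
; Only one group is handled per tick, and none is restored.
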(event EventBeginPlay
  (bind _outactors (Actor|GetAllActorsOfClass "/Game/Blueprints/BP_Pawn.BP_Pawn_C"))
  (Variables|Default|SetLife (Utilities|Array|Get(acopy) _outactors)))

(event Collision|EventActorBeginOverlap
  (params (OtherActor :type Actor%20Object%20Reference)))

(event EventTick
  (params (DeltaSeconds :type Float%20%28single-precision%29))
  (if (<= (Variables|/Game/Blueprints/BP_Pawn.BP_Pawn_C|GetLife (Variables|Default|GetLife)) 2)
    (if (<= (Variables|/Game/Blueprints/BP_Pawn.BP_Pawn_C|GetLife (Variables|Default|GetLife)) 1)
      (if (<= (Variables|/Game/Blueprints/BP_Pawn.BP_Pawn_C|GetLife (Variables|Default|GetLife)) 0)
        (if (Variables|Default|GetLife_1)
          (Components|DestroyComponent (Variables|Default|GetCube1))
          (Variables|Default|SetLife_1 false))
        (elif (Variables|Default|GetLife_2)
          (Components|DestroyComponent (Variables|Default|GetCube5))
          (Variables|Default|SetLife_2 false)))
      (elif (Variables|Default|GetLife_3)
        (Components|DestroyComponent (Variables|Default|GetCube8))
        (Variables|Default|SetLife_3 false)))))

(fn ConstructionScript)