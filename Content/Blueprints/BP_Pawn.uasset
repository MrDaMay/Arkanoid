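; BP_Pawn is the player paddle of a ball-and-bonus game, moved along X by the MoveRight axis, with keys to launch, restart or quit.
; It spawns BP_Ball, holds it on a Sphere anchor until Space sets Launch, and binds its OnDead event to spend a life and respawn.
; Bonus overlaps grow or shrink the paddle Cube within scale limits.
; When lives run out, it spawns BP_Lose and moves the camera.
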(event Custom|OnDeadReaction
  (Variables|/Game/Blueprints/BP_Ball.BP_Ball_C|SetLaunch (Variables|Default|GetPlayingBall) false)
  (Variables|Default|SetLive false)
  (bind _result (Math|Integer|DecrementInt (Variables|Default|GetLife))
    (:%20%20
      (Variables|Default|SetLife _result)
      (if (> (Variables|Default|GetLife) 0)
        (CallFunction|SpawnBall)
        (EventDispatchers|AssignOnDead (Variables|Default|GetPlayingBall) (delegate Custom|OnDeadReaction))
        (else
          (Game|SpawnActorfromClass "/Game/Blueprints/BP_Lose.BP_Lose_C" (Math|Transform|MakeTransform "-2095.000000,-55.000000,155.000000" "0,-180.000000, 0" "1,1,1") "AlwaysSpawn" 0 0)
          (Transformation|SetActorLocation (Variables|Default|GetCameraActor) "-2060.000000,-70.000000,830.000000" true false))))))

(event EventBeginPlay
  (bind _asbp_score (Utilities|Casting|CastToBP_Score (Game|GetGameInstance)))
  (Variables|Default|SetScore _asbp_score)
  (bind _outactors (Actor|GetAllActorsOfClass "/Script/Engine.CameraActor"))
  (Variables|Default|SetCameraActor (Utilities|Array|Get(acopy) _outactors))
  (if (> (Variables|Default|GetLife) 0)
    (CallFunction|SpawnBall)
    (EventDispatchers|AssignOnDead (Variables|Default|GetPlayingBall) (delegate Custom|OnDeadReaction))
    (else
      (Game|SpawnActorfromClass "/Game/Blueprints/BP_Lose.BP_Lose_C" (Math|Transform|MakeTransform "-2095.000000,-55.000000,155.000000" "0,-180.000000, 0" "1,1,1") "AlwaysSpawn" 0 0)
      (Transformation|SetActorLocation (Variables|Default|GetCameraActor) "-2060.000000,-70.000000,830.000000" true false))))

(event Collision|EventActorBeginOverlap
  (params (OtherActor :type Actor%20Object%20Reference))
  (bind _cube (Variables|Default|GetCube))
  (bind _cube_2 (Variables|Default|GetCube))
  (bind _cube_3 (Variables|Default|GetCube))
  (bind _returnvalue (Transformation|GetWorldScale _cube))
  (bind _returnvalue_2 (Transformation|GetWorldTransform _cube_2))
  (bind _returnvalue_3 (Transformation|GetWorldTransform _cube_3))
  (if (and (> (.z _returnvalue) 1.5) (< (.z _returnvalue) 4.0))
    (Utilities|Casting|CastToBP_Bonus1 OtherActor
      (:then
        (Transformation|SetWorldTransform (Variables|Default|GetCube) (Math|Transform|MakeTransform (.location _returnvalue_3) (.rotation _returnvalue_3) (+ (.scale _returnvalue_3) "0, 0,0.500000")) true false))
      (:CastFailed
        (Utilities|Casting|CastToBP_Bonus2 OtherActor)
        (Transformation|SetWorldTransform (Variables|Default|GetCube) (Math|Transform|MakeTransform (.location _returnvalue_2) (.rotation _returnvalue_2) (- (.scale _returnvalue_2) "0, 0,0.500000")) true false)))))

(event EventTick
  (params (DeltaSeconds :type Float%20%28single-precision%29))
  (bind _sphere (Variables|Default|GetSphere))
  (bind _returnvalue (Transformation|GetWorldTransform _sphere))
  (if (== (Variables|Default|GetN-Right) 1.0)
    (Transformation|AddActorWorldOffset (Math|Vector|MakeVector (* DeltaSeconds -1.5e+03) 0.0 0.0) true)
    (elif (== (Variables|Default|GetN-Left) 1.0)
      (Transformation|AddActorWorldOffset (Math|Vector|MakeVector (* DeltaSeconds 1.5e+03) 0.0 0.0) true)))
  (if (Variables|Default|GetLive)
    (if (not (Variables|/Game/Blueprints/BP_Ball.BP_Ball_C|GetLaunch (Variables|Default|GetPlayingBall)))
      (Transformation|SetActorTransform (Variables|Default|GetPlayingBall) (Math|Transform|MakeTransform (.location _returnvalue) (.rotation _returnvalue) (Transformation|GetWorldScale (Variables|/Script/Engine.Actor|GetRootComponent (Variables|Default|GetPlayingBall)))) true))))

(event Input|AxisEvents|InputAxisMoveRight
  (params (AxisValue :type Float%20%28single-precision%29))
  (if (> AxisValue 0.0)
    (Variables|Default|SetN-Right 1.0)
    (Variables|Default|SetN-Left 0.0)))

(event Input|AxisEvents|InputAxisMoveRight
  (params (AxisValue :type Float%20%28single-precision%29))
  (if (< AxisValue 0.0)
    (Variables|Default|SetN-Right 0.0)
    (Variables|Default|SetN-Left 1.0)))

(event Input|AxisEvents|InputAxisMoveRight
  (params (AxisValue :type Float%20%28single-precision%29))
  (if (== AxisValue 0.0)
    (Variables|Default|SetN-Right 0.0)
    (Variables|Default|SetN-Left 0.0)))

(event Input|KeyboardEvents|SpaceBar
  (params (Key :type Key%20Structure :default "None"))
  (:Pressed
    (Variables|/Game/Blueprints/BP_Ball.BP_Ball_C|SetLaunch (Variables|Default|GetPlayingBall) true)))

(event Input|KeyboardEvents|Escape
  (params (Key :type Key%20Structure :default "None"))
  (:Pressed
    (Game|QuitGame 0 "Quit" false)))

(event Input|KeyboardEvents|Enter
  (params (Key :type Key%20Structure :default "None"))
  (:Pressed
    (Variables|/Game/Blueprints/BP_Score.BP_Score_C|SetScore (Variables|Default|GetScore) 0)
    (Game|OpenLevel(byName) "Level_1")))

(fn ConstructionScript)

(fn SpawnBall
  (bind _sphere (Variables|Default|GetSphere))
  (bind _returnvalue (Transformation|GetWorldTransform _sphere))
  (bind _returnvalue_2 (Game|SpawnActorfromClass "/Game/Blueprints/BP_Ball.BP_Ball_C" (Math|Transform|MakeTransform (.location _returnvalue) (.rotation _returnvalue) "0.350000,0.350000,0.350000") "AlwaysSpawn" 0 0))
  (Variables|Default|SetLive true)
  (bind _output_get (Variables|Default|SetPlayingBall _returnvalue_2))
  (return _output_get))