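; Level 3 block spawner that lays out a patterned wall of blocks and handles level completion.
; On BeginPlay, nested loops walk an X-by-Y grid, using hard-coded coordinate tests to skip cells or pick one of three block classes in layers.
; Each spawn increments LivesBlocks.
; While that count is zero, Tick spawns BP_Finish_2 and moves the first found CameraActor to a fixed position, with no run-once guard.
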(event EventBeginPlay
  (bind _outactors (Actor|GetAllActorsOfClass "/Script/Engine.CameraActor"))
  (Variables|Default|SetCameraActor (Utilities|Array|Get(acopy) _outactors))
  (Variables|Default|SetChecklevel true)
  (for _index (range 1 (Variables|Default|GetX))
    (Variables|Default|SetNumb_X _index)
    (for _index_2 (range 1 (Variables|Default|GetY))
      (Variables|Default|SetNumb_Y _index_2)
      (if (not (Math|Boolean|ORBoolean (and (== (Variables|Default|GetNumb_Y) 1) (Math|Boolean|ORBoolean (== (Variables|Default|GetNumb_X) 2) (== (Variables|Default|GetNumb_X) 6) (== (Variables|Default|GetNumb_X) 10))) (== (Variables|Default|GetNumb_X) 1) (== (Variables|Default|GetNumb_X) 11) (and (== (Variables|Default|GetNumb_Y) 11) (!= (Variables|Default|GetNumb_X) 6)) (and (== (Variables|Default|GetNumb_Y) 10) (Math|Boolean|ANDBoolean (!= (Variables|Default|GetNumb_X) 5) (!= (Variables|Default|GetNumb_X) 6) (!= (Variables|Default|GetNumb_X) 7))) (and (== (Variables|Default|GetNumb_Y) 9) (Math|Boolean|ORBoolean (== (Variables|Default|GetNumb_X) 2) (== (Variables|Default|GetNumb_X) 3) (== (Variables|Default|GetNumb_X) 9) (== (Variables|Default|GetNumb_X) 10))) (and (or (== (Variables|Default|GetNumb_X) 2) (== (Variables|Default|GetNumb_X) 10)) (== (Variables|Default|GetNumb_Y) 8))))
        (if (Math|Boolean|ORBoolean (Math|Boolean|ORBoolean (== (Variables|Default|GetNumb_Y) 1) (== (Variables|Default|GetNumb_Y) 2) (== (Variables|Default|GetNumb_Y) 10) (== (Variables|Default|GetNumb_Y) 11)) (Math|Boolean|ORBoolean (== (Variables|Default|GetNumb_X) 2) (== (Variables|Default|GetNumb_X) 3) (== (Variables|Default|GetNumb_X) 9) (== (Variables|Default|GetNumb_X) 10)) (and (== (Variables|Default|GetNumb_Y) 9) (!= (Variables|Default|GetNumb_X) 6)) (and (== (Variables|Default|GetNumb_Y) 3) (== (Variables|Default|GetNumb_X) 6)) (and (== (Variables|Default|GetNumb_Y) 8) (or (== (Variables|Default|GetNumb_X) 4) (== (Variables|Default|GetNumb_X) 8))))
          (bind _result (Math|Integer|IncrementInt (Variables|Default|GetLivesBlocks))
            (:%20%20
              (Variables|Default|SetLivesBlocks _result)
              (Game|SpawnActorfromClass "/Game/Blueprints/BP_CubeBLock3.BP_CubeBLock3_C" (Math|Transform|MakeTransform (Math|Vector|MakeVector (Math|Conversions|ToFloat(Integer) (* (* _index (Variables|Default|GetPadding_X)) -1)) (Math|Conversions|ToFloat(Integer) (* (* _index_2 (Variables|Default|GetPadding_Y)) -1)) 0.0) "0, 0, 0" "1.400000,0.700000,0.700000") "Undefined" 0 0)))
          (elif (Math|Boolean|ORBoolean (or (== (Variables|Default|GetNumb_X) 4) (== (Variables|Default|GetNumb_X) 8)) (or (== (Variables|Default|GetNumb_Y) 3) (== (Variables|Default|GetNumb_Y) 9)) (and (== (Variables|Default|GetNumb_Y) 8) (or (== (Variables|Default|GetNumb_X) 5) (== (Variables|Default|GetNumb_X) 7))) (and (== (Variables|Default|GetNumb_Y) 4) (== (Variables|Default|GetNumb_X) 6)))
            (bind _result_2 (Math|Integer|IncrementInt (Variables|Default|GetLivesBlocks))
              (:%20%20
                (Variables|Default|SetLivesBlocks _result_2)
                (Game|SpawnActorfromClass "/Game/Blueprints/BP_CubeBLock2.BP_CubeBLock2_C" (Math|Transform|MakeTransform (Math|Vector|MakeVector (Math|Conversions|ToFloat(Integer) (* (* _index (Variables|Default|GetPadding_X)) -1)) (Math|Conversions|ToFloat(Integer) (* (* _index_2 (Variables|Default|GetPadding_Y)) -1)) 0.0) "0, 0, 0" "1.400000,0.700000,0.700000") "Undefined" 0 0)))
            (else
              (bind _result_3 (Math|Integer|IncrementInt (Variables|Default|GetLivesBlocks))
                (:%20%20
                  (Variables|Default|SetLivesBlocks _result_3)
                  (Game|SpawnActorfromClass "/Game/Blueprints/BP_CubeBLock1.BP_CubeBLock1_C" (Math|Transform|MakeTransform (Math|Vector|MakeVector (Math|Conversions|ToFloat(Integer) (* (* _index (Variables|Default|GetPadding_X)) -1)) (Math|Conversions|ToFloat(Integer) (* (* _index_2 (Variables|Default|GetPadding_Y)) -1)) 0.0) "0, 0, 0" "1.400000,0.700000,0.700000") "Undefined" 0 0))))))))))

(event Collision|EventActorBeginOverlap
  (params (OtherActor :type Actor%20Object%20Reference)))

(event EventTick
  (params (DeltaSeconds :type Float%20%28single-precision%29))
  (if (== (Variables|Default|GetLivesBLocks) 0)
    (Game|SpawnActorfromClass "/Game/Blueprints/BP_Finish_2.BP_Finish_2_C" (Math|Transform|MakeTransform "-2095.000000,-55.000000,155.000000" "0,-180.000000, 0" "1,1,1") "AlwaysSpawn" 0 0)
    (Transformation|SetActorLocation (Variables|Default|GetCameraActor) "-2060.000000,-70.000000,830.000000" true false)))

(fn ConstructionScript)