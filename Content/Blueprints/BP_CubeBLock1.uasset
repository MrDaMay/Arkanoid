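; Breakable brick for a ball-and-blocks game that is destroyed when a BP_Ball hits it.
; On BeginPlay it caches BP_Score from the game instance and finds the block managers for levels 1 to 3.
; Each hit adds a point and may spawn one of two rare bonus pickups at the cube.
; It then decrements LivesBlocks on the manager chosen by the CheckLevel flags, falling back to level 3.
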(event EventBeginPlay
  (bind _asbp_score (Utilities|Casting|CastToBP_Score (Game|GetGameInstance)))
  (Variables|Default|SetScore _asbp_score)
  (bind _returnvalue (Actor|GetActorOfClass "/Game/Blueprints/BP_BlocksForLevel_1.BP_BlocksForLevel_1_C"))
  (Variables|Default|SetBlockForLevel1 _returnvalue)
  (bind _returnvalue_2 (Actor|GetActorOfClass "/Game/Blueprints/BP_BlocksForLevel_2.BP_BlocksForLevel_2_C"))
  (Variables|Default|SetBlockForLevel2 _returnvalue_2)
  (bind _returnvalue_3 (Actor|GetActorOfClass "/Game/Blueprints/BP_BlocksForLevel_3.BP_BlocksForLevel_3_C"))
  (Variables|Default|SetBlockForLevel3 _returnvalue_3))

(event Collision|EventActorBeginOverlap
  (params (OtherActor :type Actor%20Object%20Reference)))

(event EventTick
  (params (DeltaSeconds :type Float%20%28single-precision%29)))

(event Collision|EventHit
  (params (MyComp :type Primitive%20Component%20Object%20Reference) (Other :type Actor%20Object%20Reference) (OtherComp :type Primitive%20Component%20Object%20Reference) (bSelfMoved :type Boolean) (HitLocation :type Vector :default "0, 0, 0") (HitNormal :type Vector :default "0, 0, 0") (NormalImpulse :type Vector :default "0, 0, 0") (Hit :type Hit%20Result%20Structure%20%28by%20ref%29))
  (Utilities|Casting|CastToBP_Ball Other)
  (Variables|/Game/Blueprints/BP_Score.BP_Score_C|SetScore (Variables|Default|GetScore) (+ (Variables|/Game/Blueprints/BP_Score.BP_Score_C|GetScore (Variables|Default|GetScore)) 1))
  (if (> (Math|Random|RandomIntegerinRange 1 100) 97)
    (Game|SpawnActorfromClass "/Game/Blueprints/BP_Bonus1.BP_Bonus1_C" (Math|Transform|MakeTransform (Transformation|GetWorldLocation (Variables|Default|GetCube)) "90.000000, 0, 0" "0.250000,0.250000,0.900000") "Undefined" 0 0)
    (if (Variables|/Game/Blueprints/BP_BlocksForLevel_1.BP_BlocksForLevel_1_C|GetCheckLevel (Variables|Default|GetBlockForLevel1))
      (bind _result (Math|Integer|DecrementInt (Variables|/Game/Blueprints/BP_BlocksForLevel_1.BP_BlocksForLevel_1_C|GetLivesBlocks (Variables|Default|GetBlockForLevel1)))
        (:%20%20
          (Variables|/Game/Blueprints/BP_BlocksForLevel_1.BP_BlocksForLevel_1_C|SetLivesBlocks (Variables|Default|GetBlockForLevel1) _result)))
      (elif (Variables|/Game/Blueprints/BP_BlocksForLevel_2.BP_BlocksForLevel_2_C|GetCheckLevel (Variables|Default|GetBlockForLevel2))
        (bind _result_2 (Math|Integer|DecrementInt (Variables|/Game/Blueprints/BP_BlocksForLevel_2.BP_BlocksForLevel_2_C|GetLivesBlocks (Variables|Default|GetBlockForLevel2)))
          (:%20%20
            (Variables|/Game/Blueprints/BP_BlocksForLevel_2.BP_BlocksForLevel_2_C|SetLivesBlocks (Variables|Default|GetBlockForLevel2) _result_2)))
        (else
          (bind _result_3 (Math|Integer|DecrementInt (Variables|/Game/Blueprints/BP_BlocksForLevel_3.BP_BlocksForLevel_3_C|GetLivesBLocks (Variables|Default|GetBlockForLevel3)))
            (:%20%20
              (Variables|/Game/Blueprints/BP_BlocksForLevel_3.BP_BlocksForLevel_3_C|SetLivesBLocks (Variables|Default|GetBlockForLevel3) _result_3))))))
    (Actor|DestroyActor)
    (elif (> (Math|Random|RandomIntegerinRange 1 100) 95)
      (Game|SpawnActorfromClass "/Game/Blueprints/BP_Bonus2.BP_Bonus2_C" (Math|Transform|MakeTransform (Transformation|GetWorldLocation (Variables|Default|GetCube)) "90.000000, 0, 0" "0.250000,0.250000,0.900000") "Undefined" 0 0)
      (if (Variables|/Game/Blueprints/BP_BlocksForLevel_1.BP_BlocksForLevel_1_C|GetCheckLevel (Variables|Default|GetBlockForLevel1))
        (bind _result_4 (Math|Integer|DecrementInt (Variables|/Game/Blueprints/BP_BlocksForLevel_1.BP_BlocksForLevel_1_C|GetLivesBlocks (Variables|Default|GetBlockForLevel1)))
          (:%20%20
            (Variables|/Game/Blueprints/BP_BlocksForLevel_1.BP_BlocksForLevel_1_C|SetLivesBlocks (Variables|Default|GetBlockForLevel1) _result_4)))
        (elif (Variables|/Game/Blueprints/BP_BlocksForLevel_2.BP_BlocksForLevel_2_C|GetCheckLevel (Variables|Default|GetBlockForLevel2))
          (bind _result_5 (Math|Integer|DecrementInt (Variables|/Game/Blueprints/BP_BlocksForLevel_2.BP_BlocksForLevel_2_C|GetLivesBlocks (Variables|Default|GetBlockForLevel2)))
            (:%20%20
              (Variables|/Game/Blueprints/BP_BlocksForLevel_2.BP_BlocksForLevel_2_C|SetLivesBlocks (Variables|Default|GetBlockForLevel2) _result_5)))
          (else
            (bind _result_6 (Math|Integer|DecrementInt (Variables|/Game/Blueprints/BP_BlocksForLevel_3.BP_BlocksForLevel_3_C|GetLivesBLocks (Variables|Default|GetBlockForLevel3)))
              (:%20%20
                (Variables|/Game/Blueprints/BP_BlocksForLevel_3.BP_BlocksForLevel_3_C|SetLivesBLocks (Variables|Default|GetBlockForLevel3) _result_6))))))
      (Actor|DestroyActor)
      (else
        (if (Variables|/Game/Blueprints/BP_BlocksForLevel_1.BP_BlocksForLevel_1_C|GetCheckLevel (Variables|Default|GetBlockForLevel1))
          (bind _result_7 (Math|Integer|DecrementInt (Variables|/Game/Blueprints/BP_BlocksForLevel_1.BP_BlocksForLevel_1_C|GetLivesBlocks (Variables|Default|GetBlockForLevel1)))
            (:%20%20
              (Variables|/Game/Blueprints/BP_BlocksForLevel_1.BP_BlocksForLevel_1_C|SetLivesBlocks (Variables|Default|GetBlockForLevel1) _result_7)))
          (elif (Variables|/Game/Blueprints/BP_BlocksForLevel_2.BP_BlocksForLevel_2_C|GetCheckLevel (Variables|Default|GetBlockForLevel2))
            (bind _result_8 (Math|Integer|DecrementInt (Variables|/Game/Blueprints/BP_BlocksForLevel_2.BP_BlocksForLevel_2_C|GetLivesBlocks (Variables|Default|GetBlockForLevel2)))
              (:%20%20
                (Variables|/Game/Blueprints/BP_BlocksForLevel_2.BP_BlocksForLevel_2_C|SetLivesBlocks (Variables|Default|GetBlockForLevel2) _result_8)))
            (else
              (bind _result_9 (Math|Integer|DecrementInt (Variables|/Game/Blueprints/BP_BlocksForLevel_3.BP_BlocksForLevel_3_C|GetLivesBLocks (Variables|Default|GetBlockForLevel3)))
                (:%20%20
                  (Variables|/Game/Blueprints/BP_BlocksForLevel_3.BP_BlocksForLevel_3_C|SetLivesBLocks (Variables|Default|GetBlockForLevel3) _result_9))))))
        (Actor|DestroyActor)))))

(fn ConstructionScript)